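; BP_OpenDoor is a door actor that swings open when enough weight rests on its PressurePlate.
; Plate overlap begin and end events re-sum the mass of overlapping static mesh actors into TotalMass.
; Tick compares that total to ComparedMass, playing OpenDoorTimeline when it is met and reversing it otherwise.
; The timeline drives the actor's yaw, and its Sound event track plays the door lock sound.
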(event OnActorBeginOverlap(PressurePlate)
  (params (OverlappedActor :type Actor%20Object%20Reference) (OtherActor :type Actor%20Object%20Reference))
  ;[1 1 1] Compute Mass when actor change
  (CallFunction|ComputeTotalMass))

(event OnActorEndOverlap(PressurePlate)
  (params (OverlappedActor :type Actor%20Object%20Reference) (OtherActor :type Actor%20Object%20Reference))
  ;[1 1 1] Compute Mass when actor change
  (CallFunction|ComputeTotalMass))

(event EventBeginPlay)

(event Collision|EventActorBeginOverlap
  (params (OtherActor :type Actor%20Object%20Reference)))

(event EventTick
  (params (DeltaSeconds :type Float%20%28single-precision%29))
  ;[1 1 1] Event Open Door
  (if (>= (Variables|Default|GetTotalMass) (Variables|Default|GetComparedMass))
    (bind _rotationz (Timeline|OpenDoorTimeline Play)
      (:Update
        (Transformation|SetActorRotation (Math|Rotator|MakeRotator 0.0 0.0 _rotationz)))
      (:Sound
        (Audio|PlaySoundatLocation "/Game/Sounds/door-lock.door-lock" (Transformation|GetActorLocation) "0, 0, 0" 1.0 1.0 0.0 0 0 0)))
    (else
      (Timeline|OpenDoorTimeline Reverse))))

(fn ConstructionScript)

(fn ComputeTotalMass
  (Variables|Default|SetTotalMass 0.0)
  (for _array_element (Collision|GetOverlappingActors (Variables|Default|GetPressurePlate) "/Script/Engine.StaticMeshActor" :!class /Script/Engine.Actor)
    (Variables|Default|SetTotalMass (+ (Variables|Default|GetTotalMass) (Physics|GetMass (Actor|GetComponentbyClass _array_element "/Script/Engine.StaticMeshComponent"))))))